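; Wall-run Blueprint that lets the player character run along walls while falling and jump off them with Space Bar.
; Tick line-traces for right and left walls, both along the right vector, then aligns yaw to the hit normal, drives forward velocity, zeroes gravity and constrains vertical movement.
; Losing the wall restores gravity and clears the constraint.
; Space launches sideways and up, briefly suspending wall-run movement, or jumps normally otherwise.
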(event `Key|SpaceBar`
  (params (Key :type "Key Structure"))
  (bind _returnvalue (`GameplayStatics.GetPlayerCharacter` 0))
  (bind (_returnvalue_x _returnvalue_y) (`KismetMathLibrary.BreakVector` (select `bool` (`self.OnRightSide`) :`false` (* (`Actor.GetActorRightVector` _returnvalue) (`self.Get Actor Right Vector Positive`)) :`true` (* (`Actor.GetActorRightVector` _returnvalue) (`self.Get Actor Right Vector Negative`)))))
  (:`Pressed`
    (if (or (`self.RightSide?`) (`self.LeftSide?`))
      (set `self.IsJumpingOffWall` true)
      (`Character.LaunchCharacter` _returnvalue (`KismetMathLibrary.MakeVector` _returnvalue_x _returnvalue_y 650.0) false true)
      (`KismetSystemLibrary.Delay` 0.2)
      (set `self.IsJumpingOffWall` false)
      (else
        (`Character.Jump` _returnvalue))))
  (:`Released`
    (`Character.StopJumping` _returnvalue)))

(event `OffWall`
  (bind _charactermovement (`Character.CharacterMovement` (`GameplayStatics.GetPlayerCharacter` 0)))
  ;[0.5828 1 0.5574] Off Wall
  (set `CharacterMovementComponent.GravityScale` 1.6 _charactermovement)
  (`MovementComponent.SetPlaneConstraintNormal` _charactermovement (0.0 0.0 0.0)))

(event `self.ReceiveTick`
  (params (DeltaSeconds :type "Float (single-precision)"))
  (bind _returnvalue (`GameplayStatics.GetPlayerCharacter` 0))
  (bind _returnvalue_2 (`GameplayStatics.GetPlayerCharacter` 0))
  (bind _returnvalue_3 (`GameplayStatics.GetPlayerCharacter` 0))
  (bind _returnvalue_4 (`GameplayStatics.GetPlayerCharacter` 0))
  (bind _returnvalue_5 (`Actor.K2_GetActorLocation` _returnvalue))
  (bind _returnvalue_6 (`Actor.K2_GetActorLocation` _returnvalue_4))
  (bind _charactermovement (`Character.CharacterMovement` _returnvalue_3))
  (bind _charactermovement_2 (`Character.CharacterMovement` _returnvalue_2))
  (bind (_returnvalue_x _returnvalue_y) (`KismetMathLibrary.BreakVector` (* (`Actor.GetActorForwardVector` _returnvalue_3) (`self.Forward Vector Float`))))
  (bind (_returnvalue_x_2 _returnvalue_y_2) (`KismetMathLibrary.BreakVector` (* (`Actor.GetActorForwardVector` _returnvalue_2) (`self.Forward Vector Float`))))
  (if (`NavMovementComponent.IsFalling` (`Character.CharacterMovement` (`GameplayStatics.GetPlayerCharacter` 0)))
    (`|ExecutionSequence`
      (:`then_0`
        (if (not (`self.LeftSide?`))
          (bind (_outhit _returnvalue_7) (`KismetSystemLibrary.LineTraceSingle` :`Start` _returnvalue_5 :`End` (+ _returnvalue_5 (* (`Actor.GetActorRightVector` _returnvalue) (`self.50`))) :`TraceChannel` "TraceTypeQuery1" :`DrawDebugType` "ForDuration"))
          (if _returnvalue_7
            (set `self.RightSide?` true)
            (set `self.OnRightSide` true)
            (if (not (`self.IsJumpingOffWall`))
              (bind (_returnvalue_roll _returnvalue_pitch _returnvalue_yaw) (`KismetMathLibrary.BreakRotator` (`KismetMathLibrary.Conv_VectorToRotator` (`.Normal` (`GameplayStatics.BreakHitResult` _outhit)))))
              (`Actor.K2_SetActorRotation` _returnvalue_3 (`KismetMathLibrary.MakeRotator` 0.0 0.0 (+ _returnvalue_yaw 90.0)) false)
              (set `MovementComponent.Velocity` (`KismetMathLibrary.MakeVector` _returnvalue_x _returnvalue_y) _charactermovement)
              (set `CharacterMovementComponent.GravityScale` 0.0 _charactermovement)
              (`MovementComponent.SetPlaneConstraintNormal` _charactermovement (0.0 0.0 1.0)))
            (else
              (set `self.RightSide?` false)
              (`self.OffWall`)))))
      (:`then_1`
        (if (not (`self.RightSide?`))
          (bind (_outhit_2 _returnvalue_8) (`KismetSystemLibrary.LineTraceSingle` :`Start` _returnvalue_6 :`End` (+ _returnvalue_6 (* (`Actor.GetActorRightVector` _returnvalue_4) (`self.-50`))) :`TraceChannel` "TraceTypeQuery1" :`DrawDebugType` "ForDuration"))
          (if _returnvalue_8
            (set `self.LeftSide?` true)
            (set `self.OnRightSide` false)
            (if (not (`self.IsJumpingOffWall`))
              (bind (_returnvalue_roll_2 _returnvalue_pitch_2 _returnvalue_yaw_2) (`KismetMathLibrary.BreakRotator` (`KismetMathLibrary.Conv_VectorToRotator` (`.Normal` (`GameplayStatics.BreakHitResult` _outhit_2)))))
              (`Actor.K2_SetActorRotation` _returnvalue_2 (`KismetMathLibrary.MakeRotator` 0.0 0.0 (+ _returnvalue_yaw_2 -90.0)) false)
              (set `MovementComponent.Velocity` (`KismetMathLibrary.MakeVector` _returnvalue_x_2 _returnvalue_y_2) _charactermovement_2)
              (set `CharacterMovementComponent.GravityScale` 0.0 _charactermovement_2)
              (`MovementComponent.SetPlaneConstraintNormal` _charactermovement_2 (0.0 0.0 1.0)))
            (else
              (set `self.LeftSide?` false)
              (`self.OffWall`))))))))